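; Base projectile Blueprint that damages the actor it hits.
; On hit, anything other than Source takes point damage along the ProjectileMovement velocity, credited to Source's instigator controller, then the projectile destroys itself.
; CheckIgnoredActors flags actors whose class equals, or is a parent of, an entry in ActorClassesToIgnore, but the hit logic never calls it.
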(event `self.ReceiveBeginPlay`)

(event `self.ReceiveHit`
  (params (MyComp :type "PrimitiveComponent Object Reference") (Other :type "Actor Object Reference") (OtherComp :type "PrimitiveComponent Object Reference") (bSelfMoved :type Boolean) (HitLocation :type "Vector Structure") (HitNormal :type "Vector Structure") (NormalImpulse :type "Vector Structure") (Hit :type "HitResult Structure (by ref)"))
  (bind _source (`self.Source`))
  (if (!= Other _source)
    (`GameplayStatics.ApplyPointDamage` Other (`self.DamageDone`) (`MovementComponent.Velocity` (`self.ProjectileMovement`)) Hit (`self.GetInstigatorController` _source) self)
    (`self.K2_DestroyActor`)))

(fn `CheckIgnoredActors`
  (params (CheckActor :type "Actor Object Reference"))
  (returns (IgnoreActor :type Boolean))
  (locals (ActorIgnored :type Boolean))
  (bind _returnvalue (`GameplayStatics.GetObjectClass` CheckActor))
  (for _array_element (`self.ActorClassesToIgnore`)
    (if (or (== _returnvalue _array_element) (`KismetMathLibrary.ClassIsChildOf` _array_element _returnvalue))
      (set `local.ActorIgnored` true)
      (return true)))
  (return false))

(fn `UserConstructionScript`)