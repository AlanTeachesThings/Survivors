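; Base Blueprint for auto-firing player abilities, owned by the survivor player.
; On BeginPlay it creates an ability widget with name and icon and adds it to the HUD's ability container.
; Tick accumulates time, updates the widget's cooldown and calls the empty Fire hook whenever the cooldown elapses.
; A FireProjectile helper spawns scaled-down projectiles at the weapon muzzle with the player as source and instigator.
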(event `self.ReceiveBeginPlay`
  (bind _output_get (set `self.PlayerREF` (cast `/Game/Characters/Base/Surv_Player_BP` (`self.GetOwner`) :!pure true)))
  (bind _returnvalue (`|CreateWidget` "/Game/Abilities/Ability_Base_W.Ability_Base_W_C" null (`self.Ability Name`) (`self.Ability Image`)))
  (bind _output_get_2 (set `self.AbilityWidget` _returnvalue))
  (`PanelWidget.AddChild` (`/Game/Characters/Base/UI/PlayerHUD_W.AbilityContainer` (`/Game/Characters/Base/Surv_Player_BP.HUD_Ref` _output_get)) _output_get_2))

(event `self.ReceiveTick`
  (params (DeltaSeconds :type "Float (single-precision)"))
  (set `self.TimeElapsed` (+ DeltaSeconds (`self.TimeElapsed`)))
  (`/Game/Abilities/Ability_Base_W.UpdateCooldown` (`self.AbilityWidget`) (/ (`self.TimeElapsed`) (`self.Cooldown`)))
  (if (> (`self.TimeElapsed`) (`self.Cooldown`))
    (`self.Fire`)
    (set `self.TimeElapsed` 0.0)))

(fn `Fire`)

(fn `FireProjectile`
  (params (ProjectileClass :type "/Game/Abilities/Base/Projectile_Base_BP Class Reference") (Rotation :type "Rotator Structure"))
  (bind _playerref (`self.PlayerREF`))
  (`|SpawnActorFromClass` ProjectileClass (`KismetMathLibrary.MakeTransform` (`SceneComponent.K2_GetComponentLocation` (`/Game/Characters/Base/Surv_Player_BP.WeaponMuzzlePoint` (`self.PlayerREF`))) Rotation (0.1 0.1 0.1)) "Undefined" "OverrideRootScale" null _playerref (`|MakeArray` "/Game/Characters/Base/Surv_Player_BP.Surv_Player_BP_C" "/Game/Characters/Base/Surv_Player_Mod_BP.Surv_Player_Mod_BP_C" :!type "Actor Class Reference") _playerref))