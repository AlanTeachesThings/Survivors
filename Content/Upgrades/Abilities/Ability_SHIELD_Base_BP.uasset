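; Base shield ability component that surrounds its owner with a damaging sphere against enemies.
; On BeginPlay it adds a visible sphere component scaled by ShieldSize to the owner and binds its begin-overlap event.
; Overlapping Enemy_Base_BP actors take point damage and are launched by a unit vector from the negated owner-to-enemy look-at rotation, with debug prints.
; Fire and Tick only call the parent.
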(event `self.ReceiveBeginPlay`
  (bind _shieldsize (`self.ShieldSize`))
  (`parent.ReceiveBeginPlay`)
  (bind _returnvalue (`|AddComponentByClass` (`self.GetOwner`) "/Script/Engine.SphereComponent" false (`KismetMathLibrary.MakeTransform` (0.0 0.0 0.0) (struct) (`KismetMathLibrary.MakeVector` _shieldsize _shieldsize _shieldsize))))
  (bind _output_get (set `self.ShieldCollider` _returnvalue))
  (add `PrimitiveComponent.OnComponentBeginOverlap` _output_get (delegate `ShieldOVerlapBegin`))
  (`SceneComponent.SetHiddenInGame` _output_get false false))

(event `self.ReceiveTick`
  (params (DeltaSeconds :type "Float (single-precision)"))
  (`parent.ReceiveTick` DeltaSeconds))

(event `ShieldOVerlapBegin`
  (params (OverlappedComponent :type "PrimitiveComponent Object Reference") (OtherActor :type "Actor Object Reference") (OtherComp :type "PrimitiveComponent Object Reference") (OtherBodyIndex :type Integer) (bFromSweep :type Boolean) (SweepResult :type "HitResult Structure (by ref)"))
  (bind _returnvalue (`Actor.K2_GetActorLocation` (`self.GetOwner`)))
  (bind _asenemy_base_bp (cast `/Game/Enemies/Enemy_Base_BP` OtherActor))
  (`KismetSystemLibrary.PrintString` (`KismetSystemLibrary.GetDisplayName` OtherComp))
  (bind _returnvalue_2 (`GameplayStatics.ApplyPointDamage` _asenemy_base_bp (`self.ShieldDamageToEnemy`) _returnvalue SweepResult (`GameplayStatics.GetPlayerController` 0) (`self.GetOwner`)))
  (`KismetSystemLibrary.PrintString` (`KismetStringLibrary.Conv_DoubleToString` _returnvalue_2))
  (`Character.LaunchCharacter` _asenemy_base_bp (`KismetMathLibrary.GreaterGreater_VectorRotator` (1.0 0.0 0.0) (`KismetMathLibrary.NegateRotator` (`KismetMathLibrary.FindLookAtRotation` _returnvalue (`Actor.K2_GetActorLocation` _asenemy_base_bp)))) false false))

(fn `Fire`
  (`parent.Fire`))