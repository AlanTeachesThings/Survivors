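; Base upgrade Blueprint for the survivor player, caching its owning Surv_Player_BP on BeginPlay.
; Fire is an empty stub, presumably for child upgrades to override.
; FireProjectile spawns a given class at the player's weapon muzzle with supplied rotation and scale, setting the player as instigator.
; FindWidgetByClass searches the HUD's ability container for a widget of an exact class and reports whether it was found.
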(event `self.ReceiveBeginPlay`
  (set `self.PlayerREF` (cast `/Game/Player/Base/Surv_Player_BP` (`self.GetOwner`) :!pure true)))

(fn `FindWidgetByClass`
  (params (WidgetClassToFind :type "/Game/Upgrades/Base/Ability_Base_W Class Reference"))
  (returns (WidgetFound :type "Widget Object Reference") (FoundWidget :type Boolean))
  (locals (Success :type Boolean) (Widget :type "Widget Object Reference"))
  (set `local.Success` false)
  (for _array_element (`PanelWidget.GetAllChildren` (`/Game/Player/Base/UI/PlayerHUD_W.AbilityContainer` (`/Game/Player/Base/Surv_Player_BP.HUD_Ref` (`self.PlayerREF`))))
    (if (== (`GameplayStatics.GetObjectClass` _array_element) WidgetClassToFind)
      (set `local.Widget` _array_element)
      (set `local.Success` true)))
  (return (`local.Widget`) (`local.Success`)))

(fn `Fire`)

(fn `FireProjectile`
  (params (ProjectileClass :type "/Game/Upgrades/Attacks/Projectile_Base_BP Class Reference") (Rotation :type "Rotator Structure") (Scale :type "Vector Structure"))
  (bind _playerref (`self.PlayerREF`))
  (`|SpawnActorFromClass` ProjectileClass (`KismetMathLibrary.MakeTransform` (`SceneComponent.K2_GetComponentLocation` (`/Game/Player/Base/Surv_Player_BP.WeaponMuzzlePoint` (`self.PlayerREF`))) Rotation Scale) "Undefined" "OverrideRootScale" null _playerref (`|MakeArray` "/Game/Player/Base/Surv_Player_BP.Surv_Player_BP_C" "/Game/Player/Base/Surv_Player_Mod_BP.Surv_Player_Mod_BP_C" :!type "Actor Class Reference") _playerref))