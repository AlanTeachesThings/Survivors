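; Homing rocket projectile for an attack upgrade that steers toward enemies and activates an explosion on hit.
; A delay loop started on BeginPlay re-runs the target search at a set interval and assigns the result as the projectile movement's homing target.
; FindNearestEnemy scans all Enemy_Base_BP actors within a fixed range, but never updates the shortest distance, so it returns the last in-range enemy rather than the nearest.
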(event `self.ReceiveBeginPlay`
  (bind (_enemyfound _nearestenemy) (`self.FindNearestEnemy`))
  (`parent.ReceiveBeginPlay`)
  (if _enemyfound :!label _label
    (set `ProjectileMovementComponent.HomingTargetComponent` (`Actor.RootComponent` _nearestenemy) (`self.ProjectileMovement`)))
  (`KismetSystemLibrary.Delay` (`self.HomingUpdateFrequency`))
  (`self.CheckForEnemy`))

(event `CheckForEnemy`
  (goto _label))

(event `self.ReceiveTick`
  (params (DeltaSeconds :type "Float (single-precision)"))
  (`parent.ReceiveTick` DeltaSeconds))

(event `self.ReceiveHit`
  (params (MyComp :type "PrimitiveComponent Object Reference") (Other :type "Actor Object Reference") (OtherComp :type "PrimitiveComponent Object Reference") (bSelfMoved :type Boolean) (HitLocation :type "Vector Structure") (HitNormal :type "Vector Structure") (NormalImpulse :type "Vector Structure") (Hit :type "HitResult Structure (by ref)"))
  (`ActorComponent.Activate` (`self.Explosion`) true)
  (`parent.ReceiveHit` MyComp Other OtherComp bSelfMoved HitLocation HitNormal NormalImpulse Hit))

(fn `FindNearestEnemy`
  (returns (EnemyFound :type Boolean) (NearestEnemy :type "/Game/Enemies/Enemy_Base_BP Object Reference"))
  (locals (ShortestDistance :type "Float (double-precision)" :default 1000.0) (NearestEnemyLocal :type "/Game/Enemies/Enemy_Base_BP Object Reference") (EnemyFoundLocal :type Boolean))
  (set `local.ShortestDistance` 1000.0)
  (set `local.EnemyFoundLocal` false)
  (bind _outactors (`GameplayStatics.GetAllActorsOfClass` "/Game/Enemies/Enemy_Base_BP.Enemy_Base_BP_C"))
  (for _array_element _outactors
    (if (< (`KismetMathLibrary.Vector_Distance` (`self.K2_GetActorLocation` _array_element) (`self.K2_GetActorLocation`)) (`local.ShortestDistance`))
      (set `local.NearestEnemyLocal` _array_element)
      (set `local.EnemyFoundLocal` true)))
  (return (`local.EnemyFoundLocal`) (`local.NearestEnemyLocal`)))

(fn `UserConstructionScript`
  (`parent.UserConstructionScript`))