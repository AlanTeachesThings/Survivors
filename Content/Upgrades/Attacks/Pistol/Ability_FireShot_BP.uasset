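; Pistol attack ability Blueprint that fires shots for the player.
; Its Fire override loops FireCount times, spawning a projectile of the configured class and scale along the player actor's rotation.
; The parent Fire runs inside the loop, once per projectile.
; BeginPlay and Tick are unused disabled stubs.
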(fn `Fire`
  (for _ (range (`self.FireCount`))
    (`self.FireProjectile` (`self.ProjectileClass`) (`Actor.K2_GetActorRotation` (`self.PlayerREF`)) (`self.ProjectileScale`))
    (`parent.Fire`)))