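; Base Blueprint for a player upgrade ability that fires automatically on a repeating cooldown.
; On BeginPlay it casts its owner to the survivor player, creates an ability widget with the name and image, and adds it to the HUD's ability container.
; Tick accumulates elapsed time to update the widget's cooldown progress, then calls Fire and resets the timer once the cooldown is exceeded.
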(event `self.ReceiveBeginPlay`
  (bind _output_get (set `self.PlayerREF` (cast `/Game/Player/Base/Surv_Player_BP` (`self.GetOwner`) :!pure true)))
  (bind _returnvalue (`|CreateWidget` "/Game/Upgrades/Base/Ability_Base_W.Ability_Base_W_C" null (`self.Ability_Name`) (`self.Ability Image`)))
  (bind _output_get_2 (set `self.AbilityWidget` _returnvalue))
  (`PanelWidget.AddChild` (`/Game/Player/Base/UI/PlayerHUD_W.AbilityContainer` (`/Game/Player/Base/Surv_Player_BP.HUD_Ref` _output_get)) _output_get_2)
  (`parent.ReceiveBeginPlay`))

(event `self.ReceiveTick`
  (params (DeltaSeconds :type "Float (single-precision)"))
  (set `self.TimeElapsed` (+ DeltaSeconds (`self.TimeElapsed`)))
  (`/Game/Upgrades/Base/Ability_Base_W.UpdateCooldown` (`self.AbilityWidget`) (/ (`self.TimeElapsed`) (`self.Cooldown`)))
  (if (> (`self.TimeElapsed`) (`self.Cooldown`))
    (`self.Fire`)
    (set `self.TimeElapsed` 0.0)
    (`parent.ReceiveTick` DeltaSeconds)))