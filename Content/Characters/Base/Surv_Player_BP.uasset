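; Base player character Blueprint for a survivors-style game, handling movement, health, damage reactions and death.
; On begin play it adds the Enhanced Input mapping, creates the HUD, attaches a rocket ability component by class and fills health.
; Damage triggers a montage call and hurt effect, then feeds a clamped health update that drives the HUD bar.
; At zero health it disables input and collision, plays a death montage and pauses animation on blend out.
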(event `TakeDamage` :!signature `self.OnTakeAnyDamage`
  (params (DamagedActor :type "Actor Object Reference") (Damage :type "Float (single-precision)") (DamageType :type "DamageType Object Reference") (InstigatedBy :type "Controller Object Reference") (DamageCauser :type "Actor Object Reference"))
  ;[1 1 1] Taking Damage
  (`|PlayMontage` (`self.Mesh`)
    (:`then`
      (`self.UpdateHealth` (* Damage -1.0) 1.0)
      (`ActorComponent.Activate` (`self.HurtEffect`) true))))

(event `self.ReceiveBeginPlay`
  (`EnhancedInputSubsystemInterface.AddMappingContext` (pcsubsystem `EnhancedInputLocalPlayerSubsystem` (`GameplayStatics.GetPlayerController` 0)) "/Game/Characters/Base/Input/DefaultMappingContext.DefaultMappingContext" 0 (struct))
  (bind _returnvalue (`|CreateWidget` "/Game/Characters/Base/UI/PlayerHUD_W.PlayerHUD_W_C"))
  (bind _output_get (set `self.HUD_Ref` _returnvalue))
  (`UserWidget.AddToViewport` _output_get 0)
  (`self.AddAbility` "/Game/Abilities/Ability_Rocket_BP.Ability_Rocket_BP_C")
  (add `self.OnTakeAnyDamage` (delegate `TakeDamage`))
  (set `self.CurrentHealth` (`self.MaxHealth`))
  (`self.UpdateHealthBar` 100.0))

(event `EnhancedInput|/Game/Characters/Base/Input/Movement_IA`
  (params (ActionValue :type "Vector2D Structure") (ElapsedSeconds :type "Float (double-precision)") (TriggeredSeconds :type "Float (double-precision)") (InputAction :type "InputAction Object Reference" :default "/Game/Characters/Base/Input/Movement_IA.Movement_IA"))
  (:`Triggered`
    (`PawnMovementComponent.AddInputVector` (`self.CharacterMovement`) (`KismetMathLibrary.MakeVector` ActionValue_X ActionValue_Y) false)))

(event `UpdateHealth`
  (params (AdditionalHealth :type "Float (double-precision)") (BarSpeed :type "Float (double-precision)"))
  (bind _mesh (`self.Mesh`))
  ;[1 1 1] Update Health
  (bind _output_get (set `self.CurrentHealth` (`KismetMathLibrary.FClamp` (+ (`self.CurrentHealth`) AdditionalHealth) 0.0 (`self.MaxHealth`))))
  (if (<= _output_get 0.0)
    (`self.UpdateHealthBar` BarSpeed)
    (`self.DisableInput` (`GameplayStatics.GetPlayerController` 0))
    (`PrimitiveComponent.SetCollisionEnabled` (`self.CapsuleComponent`) "NoCollision")
    (`|PlayMontage` _mesh "/Game/Packs/AnimStarterPack/Death_1_Montage.Death_1_Montage"
      (:`OnBlendOut`
        (set `SkeletalMeshComponent.bPauseAnims` true _mesh)))
    (else
      (`self.UpdateHealthBar` BarSpeed))))

(fn `AddAbility`
  (params (AbilityClass :type "/Game/Abilities/Ability_Base_BP Class Reference"))
  (`|AddComponentByClass` AbilityClass))

(fn `UpdateHealthBar`
  (params (BarSpeed :type "Float (double-precision)"))
  (`/Game/Characters/Base/UI/HealthBar_W.UpdateHealth` (`/Game/Characters/Base/UI/PlayerHUD_W.HealthBar_W` (`self.HUD_Ref`)) (/ (`self.CurrentHealth`) (`self.MaxHealth`)) BarSpeed))

(fn `UserConstructionScript`)