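; Base modular player character that assembles its look from interchangeable head, hair, beard, eyebrow, chest, hand and leg meshes chosen by a Style setting.
; The construction script maps each Style option to its mesh, also updating a PreviewHead component.
; BeginPlay destroys the preview head, shows the main Mesh as head and leader pose for the body parts, and snaps eyes, eyebrows, hair and beard to its head socket.
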(event `self.ReceiveBeginPlay`
  (`self.SetUpModularCharacter`)
  (`parent.ReceiveBeginPlay`))

(fn `AttachBodyParts`
  (params (BodyComponent :type "SkeletalMeshComponent Object Reference"))
  (bind _mesh (`self.Mesh`))
  (`SceneComponent.K2_SetWorldLocationAndRotation` BodyComponent (`SceneComponent.K2_GetComponentLocation` _mesh) (`SceneComponent.K2_GetComponentRotation` _mesh) false false)
  (`SkinnedMeshComponent.SetLeaderPoseComponent` BodyComponent _mesh false false))

(fn `SetUpModularCharacter`
  (bind _mesh (`self.Mesh`))
  (`ActorComponent.K2_DestroyComponent` (`self.PreviewHead`))
  (`SceneComponent.SetVisibility` (`self.Mesh`) true false)
  (`self.AttachBodyParts` (`self.Chest`))
  (`self.AttachBodyParts` (`self.Hands`))
  (`self.AttachBodyParts` (`self.Legs`))
  (`SceneComponent.K2_AttachToComponent` (`self.Eyes`) _mesh "headSocket" "SnapToTarget" "SnapToTarget" "SnapToTarget" true)
  (`SceneComponent.K2_AttachToComponent` (`self.Eyebrow`) _mesh "headSocket" "SnapToTarget" "SnapToTarget" "SnapToTarget" true)
  (`SceneComponent.K2_AttachToComponent` (`self.Hair`) _mesh "headSocket" "SnapToTarget" "SnapToTarget" "SnapToTarget" true)
  (`SceneComponent.K2_AttachToComponent` (`self.Beard`) _mesh "headSocket" "SnapToTarget" "SnapToTarget" "SnapToTarget" true))

(fn `UserConstructionScript`
  (bind (_style_head _style_hair _style_beard _style_eyebrows _style_chest _style_hands _style_legs) (break `/Game/Characters/Base/ModularStyles/ModStyle` (`self.Style`)))
  (bind _returnvalue (select `/Game/Characters/Base/ModularStyles/Head` _style_head :`NewEnumerator0` "/Game/Packs/StylizedModularChar/Meshes/Male/Face/SK_Body_Face.SK_Body_Face" :`NewEnumerator1` "/Game/Packs/StylizedModularChar/Meshes/Male/Face/SK_BodyFace_African.SK_BodyFace_African" :`NewEnumerator2` "/Game/Packs/StylizedModularChar/Meshes/Male/Face/SK_BodyFace_Asian.SK_BodyFace_Asian" :`NewEnumerator3` "/Game/Packs/StylizedModularChar/Meshes/Male/Face/SK_Soldier_Face.SK_Soldier_Face" :`NewEnumerator4` "/Game/Packs/StylizedModularChar/Meshes/Male/Face/SK_SpaceSuit_Face.SK_SpaceSuit_Face" :`NewEnumerator5` "/Game/Packs/StylizedModularChar/Meshes/Female/Face/SK_Female_Balaclava.SK_Female_Balaclava" :`NewEnumerator6` "/Game/Packs/StylizedModularChar/Meshes/Female/Face/SK_Female_SpaceSuit_Helm.SK_Female_SpaceSuit_Helm" :`NewEnumerator7` "/Game/Packs/StylizedModularChar/Meshes/Female/Face/SK_FemaleBody_AfricanFace.SK_FemaleBody_AfricanFace" :`NewEnumerator8` "/Game/Packs/StylizedModularChar/Meshes/Female/Face/SK_FemaleBody_AsianFace.SK_FemaleBody_AsianFace" :!type "SkeletalMesh Object Reference"))
  (`parent.UserConstructionScript`)
  (`|ExecutionSequence`
    (:`then_0`
      (`SkinnedMeshComponent.SetSkinnedAssetAndUpdate` (`self.Mesh`) _returnvalue true)
      (`SkinnedMeshComponent.SetSkinnedAssetAndUpdate` (`self.PreviewHead`) _returnvalue true))
    (:`then_1`
      (`StaticMeshComponent.SetStaticMesh` (`self.Hair`) (select `/Game/Characters/Base/ModularStyles/Hair` _style_hair :`NewEnumerator0` "/Game/Packs/StylizedModularChar/Meshes/Male/Hair/SM_Aviator_Hat.SM_Aviator_Hat" :`NewEnumerator1` "/Game/Packs/StylizedModularChar/Meshes/Male/Hair/SM_Hair_01.SM_Hair_01" :`NewEnumerator2` "/Game/Packs/StylizedModularChar/Meshes/Male/Hair/SM_Hair_02.SM_Hair_02" :`NewEnumerator3` "/Game/Packs/StylizedModularChar/Meshes/Male/Hair/SM_Hair_03.SM_Hair_03" :`NewEnumerator4` "/Game/Packs/StylizedModularChar/Meshes/Male/Hair/SM_Hair_04.SM_Hair_04" :`NewEnumerator6` "/Game/Packs/StylizedModularChar/Meshes/Male/Hair/SM_Cop_Hat.SM_Cop_Hat" :`NewEnumerator7` "/Game/Packs/StylizedModularChar/Meshes/Female/Hair/SM_Female_Aviator_Hat.SM_Female_Aviator_Hat" :`NewEnumerator8` "/Game/Packs/StylizedModularChar/Meshes/Female/Hair/SM_Female_Cop_Hat.SM_Female_Cop_Hat" :`NewEnumerator9` "/Game/Packs/StylizedModularChar/Meshes/Female/Hair/SM_Female_Soldier_Helmet.SM_Female_Soldier_Helmet" :`NewEnumerator10` "/Game/Packs/StylizedModularChar/Meshes/Female/Hair/SM_FemaleHair_01.SM_FemaleHair_01" :`NewEnumerator11` "/Game/Packs/StylizedModularChar/Meshes/Female/Hair/SM_FemaleHair_02.SM_FemaleHair_02" :`NewEnumerator12` "/Game/Packs/StylizedModularChar/Meshes/Female/Hair/SM_FemaleHair_03.SM_FemaleHair_03" :!type "StaticMesh Object Reference")))
    (:`then_2`
      (`StaticMeshComponent.SetStaticMesh` (`self.Beard`) (select `/Game/Characters/Base/ModularStyles/Beard` _style_beard :`NewEnumerator0` "/Game/Packs/StylizedModularChar/Meshes/Male/Hair/SM_Beard_01.SM_Beard_01" :`NewEnumerator1` "/Game/Packs/StylizedModularChar/Meshes/Male/Hair/SM_Beard_02.SM_Beard_02" :`NewEnumerator2` "/Game/Packs/StylizedModularChar/Meshes/Male/Hair/SM_Beard_03.SM_Beard_03" :`NewEnumerator3` "/Game/Packs/StylizedModularChar/Meshes/Male/Hair/SM_Beard_04.SM_Beard_04" :!type "StaticMesh Object Reference")))
    (:`then_3`
      (`StaticMeshComponent.SetStaticMesh` (`self.Eyebrow`) (select `/Game/Characters/Base/ModularStyles/Eyebrows` _style_eyebrows :`NewEnumerator0` "/Game/Packs/StylizedModularChar/Meshes/Male/Hair/SM_Eyebrow_01.SM_Eyebrow_01" :`NewEnumerator1` "/Game/Packs/StylizedModularChar/Meshes/Male/Hair/SM_Eyebrow_02.SM_Eyebrow_02" :`NewEnumerator2` "/Game/Packs/StylizedModularChar/Meshes/Male/Hair/SM_Eyebrow_03.SM_Eyebrow_03" :`NewEnumerator3` "/Game/Packs/StylizedModularChar/Meshes/Male/Hair/SM_Eyebrow_04.SM_Eyebrow_04" :`NewEnumerator4` "/Game/Packs/StylizedModularChar/Meshes/Female/Hair/SM_FemaleEyebrow_01.SM_FemaleEyebrow_01" :`NewEnumerator5` "/Game/Packs/StylizedModularChar/Meshes/Female/Hair/SM_FemaleEyebrow_02.SM_FemaleEyebrow_02" :`NewEnumerator6` "/Game/Packs/StylizedModularChar/Meshes/Female/Hair/SM_FemaleEyebrow_03.SM_FemaleEyebrow_03" :!type "StaticMesh Object Reference")))
    (:`then_4`
      (`SkinnedMeshComponent.SetSkinnedAssetAndUpdate` (`self.Chest`) (select `/Game/Characters/Base/ModularStyles/Chest` _style_chest :`NewEnumerator0` "/Game/Packs/StylizedModularChar/Meshes/Male/Chest/SK_Aviator_Chest.SK_Aviator_Chest" :`NewEnumerator1` "/Game/Packs/StylizedModularChar/Meshes/Male/Chest/SK_Body_Chest.SK_Body_Chest" :`NewEnumerator2` "/Game/Packs/StylizedModularChar/Meshes/Male/Chest/SK_Casual_Chest.SK_Casual_Chest" :`NewEnumerator3` "/Game/Packs/StylizedModularChar/Meshes/Male/Chest/SK_Cop_Chest.SK_Cop_Chest" :`NewEnumerator4` "/Game/Packs/StylizedModularChar/Meshes/Male/Chest/SK_Smoking_Chest.SK_Smoking_Chest" :`NewEnumerator5` "/Game/Packs/StylizedModularChar/Meshes/Male/Chest/SK_Soldier_Chest.SK_Soldier_Chest" :`NewEnumerator6` "/Game/Packs/StylizedModularChar/Meshes/Male/Chest/SK_Soldier_Chest.SK_Soldier_Chest" :`NewEnumerator7` "/Game/Packs/StylizedModularChar/Meshes/Female/Chest/SK_Female_Aviator_Chest.SK_Female_Aviator_Chest" :`NewEnumerator8` "/Game/Packs/StylizedModularChar/Meshes/Female/Chest/SK_Female_Body_Chest.SK_Female_Body_Chest" :`NewEnumerator9` "/Game/Packs/StylizedModularChar/Meshes/Female/Chest/SK_Female_Cop_Chest.SK_Female_Cop_Chest" :`NewEnumerator10` "/Game/Packs/StylizedModularChar/Meshes/Female/Chest/SK_Female_Soldier_Chest.SK_Female_Soldier_Chest" :`NewEnumerator11` "/Game/Packs/StylizedModularChar/Meshes/Female/Chest/SK_Female_SpaceSuit_Chest.SK_Female_SpaceSuit_Chest" :`NewEnumerator12` "/Game/Packs/StylizedModularChar/Meshes/Female/Chest/Tailleur_Chest.Tailleur_Chest" :!type "SkeletalMesh Object Reference") true))
    (:`then_5`
      (`SkinnedMeshComponent.SetSkinnedAssetAndUpdate` (`self.Hands`) (select `/Game/Characters/Base/ModularStyles/Hands` _style_hands :`NewEnumerator0` "/Game/Packs/StylizedModularChar/Meshes/Male/Hands/SK_Body_Hands.SK_Body_Hands" :`NewEnumerator1` "/Game/Packs/StylizedModularChar/Meshes/Male/Hands/SK_Casual_Hands.SK_Casual_Hands" :`NewEnumerator2` "/Game/Packs/StylizedModularChar/Meshes/Male/Hands/SK_SpaceSuit_Hands.SK_SpaceSuit_Hands" :`NewEnumerator3` "/Game/Packs/StylizedModularChar/Meshes/Female/Hands/SK_Female_Body_Hands.SK_Female_Body_Hands" :`NewEnumerator4` "/Game/Packs/StylizedModularChar/Meshes/Female/Hands/SK_Female_Soldier_Hands.SK_Female_Soldier_Hands" :`NewEnumerator5` "/Game/Packs/StylizedModularChar/Meshes/Female/Hands/SK_Female_SpaceSuit_Gloves.SK_Female_SpaceSuit_Gloves" :!type "SkeletalMesh Object Reference") true))
    (:`then_6`
      (`SkinnedMeshComponent.SetSkinnedAssetAndUpdate` (`self.Legs`) (select `/Game/Characters/Base/ModularStyles/Legs` _style_legs :`NewEnumerator0` "/Game/Packs/StylizedModularChar/Meshes/Male/Legs/SK_Aviator_Legs.SK_Aviator_Legs" :`NewEnumerator1` "/Game/Packs/StylizedModularChar/Meshes/Male/Legs/SK_Body_Legs.SK_Body_Legs" :`NewEnumerator2` "/Game/Packs/StylizedModularChar/Meshes/Male/Legs/SK_Casual_Legs.SK_Casual_Legs" :`NewEnumerator3` "/Game/Packs/StylizedModularChar/Meshes/Male/Legs/SK_Cop_Legs.SK_Cop_Legs" :`NewEnumerator4` "/Game/Packs/StylizedModularChar/Meshes/Male/Legs/SK_Smoking_Legs.SK_Smoking_Legs" :`NewEnumerator5` "/Game/Packs/StylizedModularChar/Meshes/Male/Legs/SK_Soldier_Legs.SK_Soldier_Legs" :`NewEnumerator6` "/Game/Packs/StylizedModularChar/Meshes/Male/Legs/SK_SpaceSuit_Legs.SK_SpaceSuit_Legs" :`NewEnumerator8` "/Game/Packs/StylizedModularChar/Meshes/Female/Legs/SK_Female_Aviator_Legs.SK_Female_Aviator_Legs" :`NewEnumerator9` "/Game/Packs/StylizedModularChar/Meshes/Female/Legs/SK_Female_Body_Legs.SK_Female_Body_Legs" :`NewEnumerator10` "/Game/Packs/StylizedModularChar/Meshes/Female/Legs/SK_Female_Cop_Legs.SK_Female_Cop_Legs" :`NewEnumerator11` "/Game/Packs/StylizedModularChar/Meshes/Female/Legs/SK_Female_Soldier_Legs.SK_Female_Soldier_Legs" :`NewEnumerator12` "/Game/Packs/StylizedModularChar/Meshes/Female/Legs/SK_Female_SpaceSuit_Legs.SK_Female_SpaceSuit_Legs" :`NewEnumerator13` "/Game/Packs/StylizedModularChar/Meshes/Female/Legs/Tailleur_Legs.Tailleur_Legs" :!type "SkeletalMesh Object Reference") true))))