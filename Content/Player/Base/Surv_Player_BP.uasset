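; Player character for a top-down Survivors-style game, with a camera held at a fixed offset and angle each tick.
; BeginPlay creates the HUD and adds a shield ability component; damage feeds clamped health, the health bar and death handling.
; Full experience pauses play for an upgrade menu built from the first Upgrades_DT rows.
; KillMenu resumes play and resets experience, but adds zero to CurrentLevel, so the level never rises.
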(event `self.ReceiveTick`
  (params (DeltaSeconds :type "Float (single-precision)"))
  (bind _camera (`self.Camera`))
  ;[1 1 1] Lock Camera in Position
  (`SceneComponent.K2_SetRelativeLocation` _camera (`KismetMathLibrary.GreaterGreater_VectorRotator` (-750.0 0.0 2000.0) (`KismetMathLibrary.NegateRotator` (`self.K2_GetActorRotation`))) false false)
  (`SceneComponent.K2_SetWorldRotation` _camera (struct :`Pitch` -70.0) false false))

(event `TakeDamage` :!signature `self.OnTakeAnyDamage`
  (params (DamagedActor :type "Actor Object Reference") (Damage :type "Float (single-precision)") (DamageType :type "DamageType Object Reference") (InstigatedBy :type "Controller Object Reference") (DamageCauser :type "Actor Object Reference"))
  ;[1 1 1] Taking Damage
  (`|PlayMontage` (`self.Mesh`)
    (:`then`
      (`self.UpdateHealth` (* Damage -1.0) 1.0)
      (`ActorComponent.Activate` (`self.HurtEffect`) true))))

(event `self.ReceiveBeginPlay`
  ;[1 1 1] BeginPlay
  (`EnhancedInputSubsystemInterface.AddMappingContext` (pcsubsystem `EnhancedInputLocalPlayerSubsystem` (`GameplayStatics.GetPlayerController` 0)) "/Game/Player/Base/Input/DefaultMappingContext.DefaultMappingContext" 0 (struct))
  (bind _returnvalue (`|CreateWidget` "/Game/Player/Base/UI/PlayerHUD_W.PlayerHUD_W_C"))
  (bind _output_get (set `self.HUD_Ref` _returnvalue))
  (`UserWidget.AddToViewport` _output_get 0)
  (`self.AddNewAbility` "/Game/Upgrades/Abilities/Ability_SHIELD_Base_BP.Ability_SHIELD_Base_BP_C")
  (add `self.OnTakeAnyDamage` (delegate `TakeDamage`))
  (set `self.CurrentHealth` (`self.MaxHealth`))
  (`self.UpdateHealthBar` 100.0))

(event `UpdateHealth`
  (params (AdditionalHealth :type "Float (double-precision)") (BarSpeed :type "Float (double-precision)"))
  (bind _mesh (`self.Mesh`))
  ;[1 1 1] Update Health
  (bind _output_get (set `self.CurrentHealth` (`KismetMathLibrary.FClamp` (+ (`self.CurrentHealth`) AdditionalHealth) 0.0 (`self.MaxHealth`))))
  (if (<= _output_get 0.0)
    (`self.UpdateHealthBar` BarSpeed)
    (`self.DisableInput` (`GameplayStatics.GetPlayerController` 0))
    (`PrimitiveComponent.SetCollisionEnabled` (`self.CapsuleComponent`) "NoCollision")
    (`|PlayMontage` _mesh "/Game/Packs/AnimStarterPack/Death_1_Montage.Death_1_Montage"
      (:`OnBlendOut`
        (set `SkeletalMeshComponent.bPauseAnims` true _mesh)))
    (else
      (`self.UpdateHealthBar` BarSpeed))))

(event `EnhancedInput|/Game/Player/Base/Input/Movement_IA`
  (params (ActionValue :type "Vector2D Structure") (ElapsedSeconds :type "Float (double-precision)") (TriggeredSeconds :type "Float (double-precision)") (InputAction :type "InputAction Object Reference" :default "/Game/Player/Base/Input/Movement_IA.Movement_IA"))
  ;[1 1 1] Movement
  (:`Triggered`
    (`PawnMovementComponent.AddInputVector` (`self.CharacterMovement`) (`KismetMathLibrary.MakeVector` ActionValue_X ActionValue_Y) false)))

(event `AddExperience`
  (params (ExperienceToAdd :type Integer))
  (bind _returnvalue (`GameplayStatics.GetPlayerController` 0))
  (bind _experiencetonextlevel (`self.ExperienceToNextLevel`))
  ;[1 1 1] Add Expereince and Check for Next Level
  (bind _output_get (set `self.CurrentExperience` (+ ExperienceToAdd (`self.CurrentExperience`))))
  (`|ExecutionSequence`
    (:`then_0`
      (`/Game/Player/Base/UI/ExperienceBar_W.UpdateExperience` (`/Game/Player/Base/UI/PlayerHUD_W.ExperienceBar_W` (`self.HUD_Ref`)) (/ (`KismetMathLibrary.Conv_IntToDouble` _output_get) (`KismetMathLibrary.Conv_IntToDouble` _experiencetonextlevel)) 1.0 (`self.CurrentExperience`) _experiencetonextlevel (`self.CurrentLevel`)))
    (:`then_1`
      (if (>= _output_get (`self.ExperienceToNextLevel`))
        (`GameplayStatics.SetGamePaused` true)
        (bind _returnvalue_2 (`|CreateWidget` "/Game/Upgrades/UI/UpgradeMenu_W.UpgradeMenu_W_C"))
        (bind _output_get_2 (set `self.AbilityMenuREF` _returnvalue_2))
        (for _index (range (`self.AbilitiesToShowInMenu`))
          (bind _outrownames (`DataTableFunctionLibrary.GetDataTableRowNames` "/Game/Upgrades/Upgrades_DT.Upgrades_DT"))
          (bind _returnvalue_3 (`|GetDataTableRow` "/Game/Upgrades/Upgrades_DT.Upgrades_DT" (`|GetArrayItem` _outrownames _index))
            (:`then`
              (bind _returnvalue_4 (`|CreateWidget` "/Game/Upgrades/UI/AbilityMenuButton_W.AbilityMenuButton_W_C" null (break `/Game/Upgrades/Upgrade` _returnvalue_3) (`.UpgradeDescription_6_98441DF64B2F5D261586C9A59541F619` (break `/Game/Upgrades/Upgrade` _returnvalue_3)) (`.UpgradeClass_14_8CB7423945A964A89C7C1ABBFBC6AFB6` (break `/Game/Upgrades/Upgrade` _returnvalue_3))))
              (`PanelWidget.AddChild` (`/Game/Upgrades/UI/UpgradeMenu_W.AbilityButtonContainer` (`self.AbilityMenuREF`)) _returnvalue_4))))
        (`UserWidget.AddToViewport` _output_get_2 0)
        (`WidgetBlueprintLibrary.SetInputMode_UIOnlyEx` _returnvalue (`PanelWidget.GetChildAt` (`/Game/Upgrades/UI/UpgradeMenu_W.AbilityButtonContainer` (`self.AbilityMenuREF`)) 0))
        (set `PlayerController.bShowMouseCursor` true _returnvalue)))))

(event `KillMenu`
  (bind _returnvalue (`GameplayStatics.GetPlayerController` 0))
  (bind _experiencetonextlevel (`self.ExperienceToNextLevel`))
  (bind _currentexperience (`self.CurrentExperience`))
  ;[1 1 1] Kill Menu & Raise Level / Reset Experience Bar
  (`Widget.RemoveFromParent` (`self.AbilityMenuREF`))
  (`WidgetBlueprintLibrary.SetInputMode_GameOnly` _returnvalue)
  (set `PlayerController.bShowMouseCursor` true _returnvalue)
  (`GameplayStatics.SetGamePaused` false)
  (set `self.CurrentExperience` 0)
  (bind _output_get (set `self.CurrentLevel` (+ (`self.CurrentLevel`) 0)))
  (set `self.ExperienceToNextLevel` (`|GetArrayItem` (`self.ExpLevels`) _output_get))
  (`/Game/Player/Base/UI/ExperienceBar_W.UpdateExperience` (`/Game/Player/Base/UI/PlayerHUD_W.ExperienceBar_W` (`self.HUD_Ref`)) (/ (`KismetMathLibrary.Conv_IntToDouble` _currentexperience) (`KismetMathLibrary.Conv_IntToDouble` _experiencetonextlevel)) 1.0 _currentexperience _experiencetonextlevel (`self.CurrentLevel`)))

(fn `AddNewAbility`
  (params (AbilityClass :type "/Game/Upgrades/Upgrade_BP Class Reference"))
  (`|AddComponentByClass` AbilityClass))

(fn `UpdateHealthBar`
  (params (BarSpeed :type "Float (double-precision)"))
  (`/Game/Player/Base/UI/HealthBar_W.UpdateHealth` (`/Game/Player/Base/UI/PlayerHUD_W.HealthBar_W` (`self.HUD_Ref`)) (/ (`self.CurrentHealth`) (`self.MaxHealth`)) BarSpeed))

(fn `UserConstructionScript`)