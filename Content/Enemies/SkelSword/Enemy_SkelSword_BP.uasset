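; Sword skeleton enemy Blueprint, a child class that adds two eye components to the parent enemy's behavior.
; The construction script snaps the eye components to the left and right eye sockets on the mesh.
; On death it destroys both eyes before running the parent death behavior, and damage handling is passed straight to the parent.
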(event `self.DoDamage`
  (`parent.DoDamage`))

(event `self.DeathBehaviours`
  (`ActorComponent.K2_DestroyComponent` (`self.EyeRight`))
  (`ActorComponent.K2_DestroyComponent` (`self.EyeLeft`))
  (`parent.DeathBehaviours`))

(fn `UserConstructionScript`
  (`parent.UserConstructionScript`)
  (`SceneComponent.K2_AttachToComponent` (`self.EyeLeft`) (`self.Mesh`) "eyeSocketL" "SnapToTarget" "SnapToTarget" "SnapToTarget" true)
  (`SceneComponent.K2_AttachToComponent` (`self.EyeRight`) (`self.Mesh`) "eyeSocketR" "SnapToTarget" "SnapToTarget" "SnapToTarget" true))