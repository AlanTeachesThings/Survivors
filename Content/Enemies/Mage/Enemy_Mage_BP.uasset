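; Mage enemy Blueprint that adds a hitscan beam spell and a neck particle effect to its parent enemy class.
; MageSpell line-traces forward from the left-hand socket, spawns a Niagara shot there and damages the hit actor.
; The beam's end parameter uses the impact point, or the trace's full range on a miss.
; The construction script attaches the neck particles to a mesh socket, and DeathBehaviours destroys them before calling the parent.
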(event `self.DeathBehaviours`
  (`ActorComponent.K2_DestroyComponent` (`self.NeckParticleSystem`))
  (`parent.DeathBehaviours`))

(event `MageSpell`
  (bind _returnvalue (`SceneComponent.GetSocketLocation` (`self.Mesh`) "hand_lSocket"))
  (bind _returnvalue_location (`KismetMathLibrary.BreakTransform` (`SceneComponent.GetSocketTransform` (`self.Mesh`) "hand_lSocket" "RTS_World")))
  (bind _returnvalue_2 (+ _returnvalue (* (`self.GetActorForwardVector`) 500.0)))
  (bind _outhit (`KismetSystemLibrary.LineTraceSingle` _returnvalue _returnvalue_2 "TraceTypeQuery2"))
  (bind _returnvalue_3 (`NiagaraFunctionLibrary.SpawnSystemAtLocation` "/Game/Enemies/Mage/MageShot_NS.MageShot_NS" _returnvalue_location))
  (`FXSystemComponent.SetVectorParameter` _returnvalue_3 "BeamEndPosition" (`KismetMathLibrary.SelectVector` (`.Location` (`GameplayStatics.BreakHitResult` _outhit)) _returnvalue_2 (`GameplayStatics.BreakHitResult` _outhit)))
  (`GameplayStatics.ApplyDamage` (`.HitActor` (`GameplayStatics.BreakHitResult` _outhit)) (`self.MageSellDamage`)))

(fn `UserConstructionScript`
  (`parent.UserConstructionScript`)
  (`SceneComponent.K2_AttachToComponent` (`self.NeckParticleSystem`) (`self.Mesh`) "neckParticleSocket" "KeepRelative" "KeepRelative" "KeepRelative" true))