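; Base enemy character that spawns with a weapon, fights the player and can drop an experience orb on death.
; After the spawn montage it runs a behaviour tree, seeding the blackboard from its behaviour settings.
; Point damage updates the health bar, stuns it, records the player and triggers fear or death with a Niagara effect.
; Movement modes set speed and facing, while an AnimBP notify damages actors tracked by box overlaps.
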(event `self.ReceiveBeginPlay`
  (bind _defaultweaponclass (`self.DefaultWeaponClass`))
  ;[1 0.8615 0] BeginPlay
  (if (`KismetSystemLibrary.IsValidClass` _defaultweaponclass)
    (bind _returnvalue (`|AddComponentByClass` _defaultweaponclass true))
    (`SceneComponent.K2_AttachToComponent` _returnvalue null "hand_rSocket" "KeepRelative" "KeepRelative" "KeepRelative" true)
    (set `self.EquippedWeapon` _returnvalue)
    (bind _returnvalue_2 (`AddComponent|NODE_AddSkeletalMeshComponent-0`))
    (bind _output_get (set `self.WeaponMesh` _returnvalue_2))
    (`SceneComponent.K2_AttachToComponent` _output_get (`self.Mesh`) "hand_rSocket" "SnapToTarget" "SnapToTarget" "SnapToTarget" true)
    (`SkinnedMeshComponent.SetSkinnedAssetAndUpdate` (`self.WeaponMesh`) (defaults `Object` _defaultweaponclass) true))
  (add `self.OnTakePointDamage` (delegate `TakePointDamage`))
  (`self.AddHealth` (`self.MaxHealth`) 1.0)
  (`|PlayMontage` (`self.Mesh`) (`self.SpawnAnim`)
    (:`OnCompleted`
      ;;[1 1 1] AI Setup
      (bind _asaicontroller (cast `AIController` (`self.GetController`)))
      (bind _output_get_2 (set `self.AIControllerREF` _asaicontroller))
      (`AIController.RunBehaviorTree` _output_get_2 (`self.BaseBehaviourTree`))
      (`self.SetupEnemyBehaviour`)
      (`self.ChangeMovementMode` "NewEnumerator0"))))

(event `TakePointDamage` :!signature `self.OnTakePointDamage`
  (params (DamagedActor :type "Actor Object Reference") (Damage :type "Float (single-precision)") (InstigatedBy :type "Controller Object Reference") (HitLocation :type "Vector Structure") (FHitComponent :type "PrimitiveComponent Object Reference") (BoneName :type Name) (ShotFromDirection :type "Vector Structure") (DamageType :type "DamageType Object Reference") (DamageCauser :type "Actor Object Reference"))
  (bind _asprojectile_base_bp (cast `/Game/Upgrades/Attacks/Projectile_Base_BP` DamageCauser :!pure true))
  (bind _aicontrollerref (`self.AIControllerREF`))
  (bind _returnvalue (`AIBlueprintHelperLibrary.GetBlackboard` (`self.AIControllerREF`)))
  (bind (_returnvalue_roll _returnvalue_pitch _returnvalue_yaw) (`KismetMathLibrary.BreakRotator` (`KismetMathLibrary.FindLookAtRotation` (`self.GetActorForwardVector`) ShotFromDirection)))
  ;[1 1 1] Take Damage
  (`self.AddHealth` (* Damage -1.0) 1.0)
  (set `self.TakeHit` true)
  (set `self.HitDirection` _returnvalue_yaw)
  (`/Engine/EditorBlueprintResources/StandardMacros.IsValid` _aicontrollerref
    (:`Is Valid`
      (`Controller.StopMovement` _aicontrollerref)
      (`BlackboardComponent.SetValueAsBool` (`AIBlueprintHelperLibrary.GetBlackboard` _aicontrollerref) "Stunned" true)
      (if (`KismetSystemLibrary.IsValid` _asprojectile_base_bp)
        (`KismetSystemLibrary.Delay` (`/Game/Upgrades/Attacks/Projectile_Base_BP.StunTime` _asprojectile_base_bp))
        (else
          (`KismetSystemLibrary.Delay` 1.0)))
      (set `self.TakeHit` false)
      (`BlackboardComponent.SetValueAsBool` _returnvalue "Stunned" false)
      (bind _assurv_player_bp (cast `/Game/Player/Base/Surv_Player_BP` (`Controller.K2_GetPawn` InstigatedBy)))
      (`BlackboardComponent.SetValueAsObject` _returnvalue "Player" _assurv_player_bp))))

(event `self.ReceiveTick`
  (params (DeltaSeconds :type "Float (single-precision)"))
  (bind (_returnvalue_roll _returnvalue_pitch) (`KismetMathLibrary.BreakRotator` (`self.K2_GetActorRotation`)))
  (bind (_asactor _bsuccess) (cast `Actor` (`BlackboardComponent.GetValueAsObject` (`AIBlueprintHelperLibrary.GetBlackboard` (`self.AIControllerREF`)) "Player") :!pure true))
  (bind (_returnvalue_roll_2 _returnvalue_pitch_2 _returnvalue_yaw) (`KismetMathLibrary.BreakRotator` (`KismetMathLibrary.FindLookAtRotation` (`self.K2_GetActorLocation`) (`self.K2_GetActorLocation` _asactor))))
  ;[0 1 0.2126] OnTick
  ;;[1 1 1] If Strfing, turn to face player (assumes ChargePlayer is set on Blackboard)
  (if (`|EnumEquality` (`self.MovementMode`) "NewEnumerator3")
    (if _bsuccess
      (`self.K2_SetActorRotation` (`KismetMathLibrary.MakeRotator` _returnvalue_roll _returnvalue_pitch _returnvalue_yaw)))))

(event `DeathBehaviours`
  (bind _mesh (`self.Mesh`))
  ;[1 1 1] Death Behaviours
  (set `self.MovementMode` "NewEnumerator0")
  (`ActorComponent.K2_DestroyComponent` (`self.HealthBar`))
  (bind _returnvalue (`NiagaraFunctionLibrary.SpawnSystemAttached` "/Game/Enemies/FX/EnemyDeathEffect.EnemyDeathEffect" _mesh "root" (0.0 0.0 0.0) (struct) "SnapToTarget" false false))
  (`NiagaraComponent.SetVariableTexture` _returnvalue "Tex" (`self.TextureForDeathEffect`))
  (`ActorComponent.Activate` _returnvalue true)
  (`SceneComponent.SetVisibility` _mesh false false)
  (`KismetSystemLibrary.Delay` 3.0)
  (if (>= (`self.ChanceToDropExp`) (`KismetMathLibrary.RandomFloatInRange` 0.0 1.0))
    (`|SpawnActorFromClass` "/Game/ExpOrb_BP.ExpOrb_BP_C" (`KismetMathLibrary.MakeTransform` (`self.K2_GetActorLocation`)) "Undefined" "OverrideRootScale" null null))
  (`self.K2_DestroyActor`))

(event `AddHealth`
  (params (AddedHealth :type "Float (double-precision)") (WidgetUpdateSpeed :type "Float (double-precision)"))
  (bind _aicontrollerref (`self.AIControllerREF`))
  (bind _mesh (`self.Mesh`))
  ;[1 1 1] AddHealth & Check For Death
  (bind _output_get (set `self.CurrentHealth` (`KismetMathLibrary.FClamp` (+ (`self.CurrentHealth`) AddedHealth) 0.0 (`self.MaxHealth`))))
  (`/Game/Player/Base/UI/HealthBar_W.UpdateHealth` (cast `/Game/Player/Base/UI/HealthBar_W` (`WidgetComponent.GetWidget` (`self.HealthBar`)) :!pure true) (/ _output_get (`self.MaxHealth`)) WidgetUpdateSpeed)
  (`|ExecutionSequence`
    (:`then_0`
      (if (<= (`self.CurrentHealth`) 0.0)
        ;;[1 1 1] Death
        (`Controller.StopMovement` _aicontrollerref)
        (`Controller.UnPossess` _aicontrollerref)
        (`|PlayMontage` _mesh (`self.DeathAnim`)
          (:`then`
            (`PrimitiveComponent.SetCollisionEnabled` (`self.CapsuleComponent`) "NoCollision")
            (set `self.MovementMode` "NewEnumerator0"))
          (:`OnBlendOut`
            (set `SkeletalMeshComponent.bPauseAnims` true _mesh)
            (`self.DeathBehaviours`)))
        (else
          ;;[1 1 1] Fear
          (if (< (`self.CurrentHealth`) (* (`self.MaxHealth`) (`self.HealthLossPercentileBeforeFear`)))
            (`BlackboardComponent.SetValueAsBool` (`AIBlueprintHelperLibrary.GetBlackboard` null) "ScaredOfPlayer" true)))))))

(event `ChangeMovementMode`
  (params (NewMovementMode :type "/Game/Enemies/MovementMode Enum" :default "NewEnumerator0"))
  (bind _charactermovement (`self.CharacterMovement`))
  ;[1 1 1] ChangeMovementMode
  (bind _output_get (set `self.MovementMode` NewMovementMode))
  (switch `/Game/Enemies/MovementMode` _output_get
    (:`NewEnumerator0`
      (set `CharacterMovementComponent.bOrientRotationToMovement` true (`self.CharacterMovement`))
      (set `CharacterMovementComponent.MaxWalkSpeed` (`self.WalkSpeed`) _charactermovement :!label _label))
    (:`NewEnumerator3`
      (set `CharacterMovementComponent.bOrientRotationToMovement` false (`self.CharacterMovement`))
      (goto _label))
    (:`NewEnumerator1`
      (set `CharacterMovementComponent.bOrientRotationToMovement` true (`self.CharacterMovement`) :!label _label_2)
      (set `CharacterMovementComponent.MaxWalkSpeed` (`self.RunSpeed`) _charactermovement))
    (:`NewEnumerator2`
      (goto _label_2))))

(event `DoDamage`
  ;[1 1 1] DoDamage: triggered by AnimBP notify event
  (for _array_element (`self.OverlappedActors`)
    (`GameplayStatics.ApplyDamage` _array_element (`self.DamageDone`) (`self.GetController`) self)))

(event `self.Box.OnComponentBeginOverlap`
  (params (OverlappedComponent :type "PrimitiveComponent Object Reference") (OtherActor :type "Actor Object Reference") (OtherComp :type "PrimitiveComponent Object Reference") (OtherBodyIndex :type Integer) (bFromSweep :type Boolean) (SweepResult :type "HitResult Structure (by ref)"))
  ;[1 1 1] Overlap System (because OverlappedActors wasn't working somehow)
  (`KismetArrayLibrary.Array_Add` (`self.OverlappedActors`) OtherActor))

(event `self.Box.OnComponentEndOverlap`
  (params (OverlappedComponent :type "PrimitiveComponent Object Reference") (OtherActor :type "Actor Object Reference") (OtherComp :type "PrimitiveComponent Object Reference") (OtherBodyIndex :type Integer))
  ;[1 1 1] Overlap System (because OverlappedActors wasn't working somehow)
  (`KismetArrayLibrary.Array_RemoveItem` (`self.OverlappedActors`) OtherActor))

(fn `Attack`
  (returns (AttackTime :type "Float (double-precision)"))
  (bind _returnvalue (`self.PlayAnimMontage` (`self.AttackAnim`)))
  (return _returnvalue))

(fn `SetAttack`
  (params (shouldAttack :type Boolean))
  (bind _output_get (set `self.shouldAttack` shouldAttack))
  (`BlackboardComponent.SetValueAsBool` (`AIBlueprintHelperLibrary.GetBlackboard` (`self.GetController`)) "isAttacking" _output_get))

(fn `SetupEnemyBehaviour`
  (bind (_enemybehaviour_chancetostalkinsteadofcharge _enemybehaviour_detectrange _enemybehaviour_meleeattackrange _enemybehaviour_longattackrange) (break `/Game/Enemies/EnemyBehaviour` (`self.EnemyBehaviour`)))
  (bind _returnvalue (`AIBlueprintHelperLibrary.GetBlackboard` (`self.AIControllerREF`)))
  (`|ExecutionSequence`
    (:`then_0`
      (`BlackboardComponent.SetValueAsFloat` _returnvalue "ChanceToStalkInsteadOfCharge" _enemybehaviour_chancetostalkinsteadofcharge))
    (:`then_1`
      (`BlackboardComponent.SetValueAsFloat` _returnvalue "PlayerDetectRange" _enemybehaviour_detectrange))
    (:`then_2`
      (`BlackboardComponent.SetValueAsFloat` _returnvalue "MeleeRange" _enemybehaviour_meleeattackrange))
    (:`then_3`
      (`BlackboardComponent.SetValueAsFloat` _returnvalue "AttackRange" _enemybehaviour_longattackrange))))

(fn `UserConstructionScript`)